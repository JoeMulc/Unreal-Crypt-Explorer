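; Lockable door actor that swings open when a released, tagged key sits inside its trigger.
; Trigger overlap events maintain an actor list that Tick scans for the key tag without a "Grabbed" tag.
; A matching key snaps to the KeyHolder socket with physics disabled, then a one-shot timeline drives the actor's relative yaw.
; BeginPlay also hands the Mover to the Trigger.
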(event OnComponentBeginOverlap(Trigger)
  (params (OverlappedComponent :type Primitive%20Component%20Object%20Reference) (OtherActor :type Actor%20Object%20Reference) (OtherComp :type Primitive%20Component%20Object%20Reference) (OtherBodyIndex :type Integer) (bFromSweep :type Boolean) (SweepResult :type Hit%20Result%20Structure%20%28by%20ref%29))
  (Utilities|Array|Add (Variables|Default|Getoverlapped%20actors) OtherActor))

(event OnComponentEndOverlap(Trigger)
  (params (OverlappedComponent :type Primitive%20Component%20Object%20Reference) (OtherActor :type Actor%20Object%20Reference) (OtherComp :type Primitive%20Component%20Object%20Reference) (OtherBodyIndex :type Integer))
  (Utilities|Array|RemoveItem (Variables|Default|Getoverlapped%20actors) OtherActor))

(event Custom|DoRotate
  (if (not (Variables|Default|GetdoRotate!))
    (Variables|Default|SetdoRotate! true)
    (bind _rotate (Timeline|rotateTimeline PlayFromStart)
      (:Update
        (Transformation|SetActorRelativeRotation (Math|Rotator|MakeRotator 0.0 0.0 _rotate))))))

(event EventBeginPlay
  (Class|TriggerComponent|SetMover (Variables|Default|GetTrigger) (Variables|Default|GetMover)))

(event Collision|EventActorBeginOverlap
  (params (OtherActor :type Actor%20Object%20Reference)))

(event EventTick
  (params (DeltaSeconds :type Float%20%28single-precision%29))
  (for _array_element (Variables|Default|Getoverlapped%20actors)
    (if (Actor|ActorHasTag _array_element (Variables|Default|GetKeyTag))
      (if (not (Actor|ActorHasTag _array_element "Grabbed"))
        (Transformation|AttachActorToActor _array_element self "KeyHolder" "SnapToTarget" "SnapToTarget" "SnapToTarget" true)
        (bind _asprimitive_component (Utilities|Casting|CastToPrimitiveComponent (Variables|/Script/Engine.Actor|GetRootComponent _array_element)))
        (Physics|SetSimulatePhysics _asprimitive_component false)
        (Physics|SetSimulatePhysics (Variables|Default|GetTrigger) false)
        (CallFunction|DoRotate)))))

(fn ConstructionScript)